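; Rhythm-game note manager actor that loads a song's beatmap on BeginPlay and starts a hard-coded music track.
; PlaySong reads the Beatmap data table row, stores resolution, time signature, scaled BPM and note map, or plays a fallback track if missing.
; The note-map loop has no body, and the Quartz clock setup and NoteSpawner lane spawning are disconnected, so no notes spawn.
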(event Custom|Every%20Quantization%20Type
  (params (ClockName :type Name) (QuantizationType :type EQuartzCommandQuantization%20Enum :default "Bar") (NumBars :type Integer) (Beat :type Integer) (BeatFraction :type Float%20%28single-precision%29)))

(event EventBeginPlay
  (CallFunction|PlaySong "Zombiesong")
  (Audio|SpawnSound2D "/Game/RythmGameInsideAZombieNightmare/MusicFiles/Rammstein_-_Deutschland.Rammstein_-_Deutschland" 0.6 1.0 0.0 0))

(event Collision|EventActorBeginOverlap
  (params (OtherActor :type Actor%20Object%20Reference)))

(event EventTick
  (params (DeltaSeconds :type Float%20%28single-precision%29)))

(fn ConstructionScript)

(fn PlaySong
  (params (SongName :type Name))
  ;[0.15 0.15 0.15 0.5] Gets Song Data From Table
  (bind _output_get (Variables|Default|SetSong%20Name SongName))
  (bind _returnvalue (Utilities|GetDataTableRow (Variables|Default|GetBeatmap) _output_get)
    (:then
      ;[0.15 0.15 0.15 0.5] Quartz Clock And Variable Configuration
      (bind _output_get_2 (Variables|Default|SetSongToPlay _returnvalue))
      ;;[0.15 0.15 0.15 0.5] Sets Song Values
      (Variables|Default|SetResolution (.resolution _output_get_2))
      (Variables|Default|SetTime%20Signature (.timesignature _output_get_2))
      (Variables|Default|SetBeats%20Per%20Minute (Math|Conversions|ToFloat(Integer) (/ (.beatsperminute _output_get_2) 1000)))
      (bind _output_get_3 (Variables|Default|SetNote%20Map (.notemap _output_get_2)))
      (Utilities|Map|ForEachLoop(Map) _output_get_3))
    (:RowNotFound
      (Audio|SpawnSound2D "/Game/RythmGameInsideAZombieNightmare/MusicFiles/In_The_End__Official_HD_Music_Video__-_Linkin_Park.In_The_End__Official_HD_Music_Video__-_Linkin_Park" 0.75 1.0 0.0 0))))