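; Controller for a zombie-infection simulation tied to a song, holding population counts, step time and the win/lose state.
; After a short startup delay it caches the note spawner, then Tick lengthens the step time once susceptibles run low.
; When the song stops it clears infected counts, triggers Win and kills non-human actors.
; Win and Lose share a game-over guard, show their widget, then load the main menu after a delay.
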(event EventBeginPlay
  (Variables|Default|SetIsGameOver false)
  (Variables|Default|SetSimulationStepTime 0.05)
  (Utilities|FlowControl|Delay 0.3)
  (bind _returnvalue (Actor|GetActorOfClass "/Game/Blueprints/BP_NoteSpawner.BP_NoteSpawner_C"))
  (Variables|Default|SetNoteSpawner _returnvalue)
  (Variables|Default|Sethas%20Initialized true))

(event Collision|EventActorBeginOverlap
  (params (OtherActor :type Actor%20Object%20Reference)))

(event EventTick
  (params (DeltaSeconds :type Float%20%28single-precision%29))
  (if (Variables|Default|Gethas%20Initialized)
    (Utilities|FlowControl|Sequence
      (:then_0
        (if (not (> (Variables|Default|GetSusceptible) 50))
          (Variables|Default|SetSimulationStepTime 1.0)))
      (:then_1
        (if (not (Variables|/Script/ZombieApocalypse.NoteSpawner|GetbIsSongPlaying (Variables|Default|GetNoteSpawner)))
          (Variables|Default|SetZombies 0)
          (Variables|Default|SetBitten 0)
          (Variables|Default|SetSimulationStepTime 2e+01)
          (Class|SimulationController|Win)
          (bind _outactors (Actor|GetAllActorsOfClass "/Game/Blueprints/BP_HumanActor.BP_HumanActor_C"))
          (for _array_element _outactors
            ;[0.15 0.15 0.15 0.5] Only kills if non-human
            (Default|Kill _array_element)))))))

(event EventWin
  (if (not (Variables|Default|GetIsGameOver))
    (Variables|Default|SetIsGameOver true)
    (bind _returnvalue (UserInterface|CreateWidget "/Game/Blueprints/WBP_Win.WBP_Win_C"))
    (UserInterface|Viewport|AddtoViewport _returnvalue 0)
    (Utilities|FlowControl|Delay 1e+01)
    (Game|OpenLevel(byName) "MainMenu")))

(event EventLose
  (if (not (Variables|Default|GetIsGameOver))
    (bind _returnvalue (UserInterface|CreateWidget "/Game/Blueprints/WBP_Lose.WBP_Lose_C"))
    (UserInterface|Viewport|AddtoViewport _returnvalue 0)
    (Variables|Default|SetIsGameOver true)
    (Utilities|FlowControl|Delay 1e+01)
    (Game|OpenLevel(byName) "MainMenu")))

(fn ConstructionScript)