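; Note manager for a music game, an unfinished prototype meant to spawn notes in time with a song.
; BeginPlay starts a 160 BPM Quartz clock, plays a 2D sound, calls StartSong and subscribes to the beat boundary once per data table row.
; SpawnNoteForRow looks up an Experimentaldatabeats row using the loop's current element.
; The BP_Note spawn, positioned from the row's BPM, is disconnected, so no notes spawn here.
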(event Custom|beat
  (params (ClockName :type Name) (QuantizationType :type EQuartzCommandQuantization%20Enum :default "Bar") (NumBars :type Integer) (Beat :type Integer) (BeatFraction :type Float%20%28single-precision%29)))

(event Custom|SpawnNoteForRow
  (params (ClockName :type Name) (QuantizationType :type EQuartzCommandQuantization%20Enum :default "Bar") (NumBars :type Integer) (Beat :type Integer) (BeatFraction :type Float%20%28single-precision%29))
  (bind _returnvalue (Utilities|GetDataTableRow "/Game/RythmGameInsideAZombieNightmare/experimentaldatabeats.experimentaldatabeats" (stale EventBeginPlay _array_element))))

(event EventBeginPlay
  (bind _returnvalue (Class|QuartzSubsystem|CreateNewClock (WorldSubsystems|GetQuartzSubsystem) "MusicClock" (Utilities|Struct|MakeQuartzClockSettings (Utilities|Struct|MakeQuartzTimeSignature 160 "QuarterNote") false) false))
  (Class|QuartzClockHandle|SetBeatsPerMinute :self _returnvalue :BeatsPerMinute 1.6e+02)
  (Variables|Default|SetActiveClockHandle _returnvalue)
  (Class|QuartzClockHandle|StartClock (Variables|Default|GetActiveClockHandle))
  (Audio|PlaySound2D 0 1.0 1.0 0.0 0 0)
  (Class|NoteManager|StartSong)
  (bind _outrownames (DataTable|GetDataTableRowNames 0))
  (for _array_element _outrownames
    (Class|QuartzClockHandle|SubscribetoQuantizationEvent (Variables|Default|GetActiveClockHandle) "Beat" (EventDispatchers|CreateEvent :!event Custom|SpawnNoteForRow))))

(event Collision|EventActorBeginOverlap
  (params (OtherActor :type Actor%20Object%20Reference)))

(event EventTick
  (params (DeltaSeconds :type Float%20%28single-precision%29)))

(fn ConstructionScript)