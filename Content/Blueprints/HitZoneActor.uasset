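; HitZoneActor is a hit zone marker that shows an arrow sprite on its Billboard component.
; The construction script checks the actor's HitZoneA, S, K and L tags and sets the matching sprite branch by branch.
; Only A maps to the same-lettered sprite; S, K and L use ArrowL, ArrowS and ArrowK respectively.
; The event graph holds only disabled placeholder events, so the actor has no runtime logic of its own.
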(event EventBeginPlay)

(event Collision|EventActorBeginOverlap
  (params (OtherActor :type Actor%20Object%20Reference)))

(event EventTick
  (params (DeltaSeconds :type Float%20%28single-precision%29)))

(fn ConstructionScript
  (Utilities|FlowControl|Sequence
    (:then_0
      (if (Actor|ActorHasTag "HitZoneA")
        (Rendering|Components|Sprite|SetSprite (Variables|Default|GetBillboard) "/Game/Sprites/ArrowA.ArrowA")))
    (:then_1
      (if (Actor|ActorHasTag "HitZoneS")
        (Rendering|Components|Sprite|SetSprite (Variables|Default|GetBillboard) "/Game/Sprites/ArrowL.ArrowL")))
    (:then_2
      (if (Actor|ActorHasTag "HitZoneK")
        (Rendering|Components|Sprite|SetSprite (Variables|Default|GetBillboard) "/Game/Sprites/ArrowS.ArrowS")))
    (:then_3
      (if (Actor|ActorHasTag "HitZoneL")
        (Rendering|Components|Sprite|SetSprite (Variables|Default|GetBillboard) "/Game/Sprites/ArrowK.ArrowK")))))