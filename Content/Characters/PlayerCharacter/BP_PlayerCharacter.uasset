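; Player character with a flipbook sprite that strikes directional poses in response to input from the IMC_Rhythm mapping context, added on BeginPlay.
; Pressing up, down, left or right swaps the sprite's flipbook to that direction, and releasing any of them restores Test_Flipbook, with no movement applied.
; Raise and lower volume inputs send fixed increments to the Game Instance through ChangeVolumeMessage.
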(event Input|EnhancedActionEvents|EnhancedInputActionIA_RaiseVolume
  (params (ActionValue :type Boolean) (ElapsedSeconds :type Float%20%28double-precision%29) (TriggeredSeconds :type Float%20%28double-precision%29) (InputAction :type Input%20Action%20Object%20Reference :default "/Game/Input/Actions/IA_RaiseVolume.IA_RaiseVolume"))
  (Class|BPIVolumeControl|ChangeVolume(Message) (Game|GetGameInstance) 0.1))

(event Input|EnhancedActionEvents|EnhancedInputActionIA_MoveDown
  (params (ActionValue :type Boolean) (ElapsedSeconds :type Float%20%28double-precision%29) (TriggeredSeconds :type Float%20%28double-precision%29) (InputAction :type Input%20Action%20Object%20Reference :default "/Game/Input/Actions/IA_MoveDown.IA_MoveDown"))
  (:Started
    (Sprite|SetFlipbook (Variables|Default|GetSprite) "/Game/Characters/PlayerCharacter/down_Flipbook.down_Flipbook"))
  (:Completed
    (Sprite|SetFlipbook (Variables|Default|GetSprite) "/Game/Characters/PlayerCharacter/Test_Flipbook.Test_Flipbook")))

(event Input|EnhancedActionEvents|EnhancedInputActionIA_MoveUp
  (params (ActionValue :type Boolean) (ElapsedSeconds :type Float%20%28double-precision%29) (TriggeredSeconds :type Float%20%28double-precision%29) (InputAction :type Input%20Action%20Object%20Reference :default "/Game/Input/Actions/IA_MoveUp.IA_MoveUp"))
  (:Started
    (Sprite|SetFlipbook (Variables|Default|GetSprite) "/Game/Characters/PlayerCharacter/up_Flipbook.up_Flipbook"))
  (:Completed
    (Sprite|SetFlipbook (Variables|Default|GetSprite) "/Game/Characters/PlayerCharacter/Test_Flipbook.Test_Flipbook")))

(event Input|EnhancedActionEvents|EnhancedInputActionIA_MoveLeft
  (params (ActionValue :type Boolean) (ElapsedSeconds :type Float%20%28double-precision%29) (TriggeredSeconds :type Float%20%28double-precision%29) (InputAction :type Input%20Action%20Object%20Reference :default "/Game/Input/Actions/IA_MoveLeft.IA_MoveLeft"))
  (:Started
    (Sprite|SetFlipbook (Variables|Default|GetSprite) "/Game/Characters/PlayerCharacter/left_Flipbook.left_Flipbook"))
  (:Completed
    (Sprite|SetFlipbook (Variables|Default|GetSprite) "/Game/Characters/PlayerCharacter/Test_Flipbook.Test_Flipbook")))

(event Input|EnhancedActionEvents|EnhancedInputActionIA_MoveRight
  (params (ActionValue :type Boolean) (ElapsedSeconds :type Float%20%28double-precision%29) (TriggeredSeconds :type Float%20%28double-precision%29) (InputAction :type Input%20Action%20Object%20Reference :default "/Game/Input/Actions/IA_MoveRight.IA_MoveRight"))
  (:Started
    (Sprite|SetFlipbook (Variables|Default|GetSprite) "/Game/Characters/PlayerCharacter/right_Flipbook.right_Flipbook"))
  (:Completed
    (Sprite|SetFlipbook (Variables|Default|GetSprite) "/Game/Characters/PlayerCharacter/Test_Flipbook.Test_Flipbook")))

(event Input|EnhancedActionEvents|EnhancedInputActionIA_LowerVolume
  (params (ActionValue :type Boolean) (ElapsedSeconds :type Float%20%28double-precision%29) (TriggeredSeconds :type Float%20%28double-precision%29) (InputAction :type Input%20Action%20Object%20Reference :default "/Game/Input/Actions/IA_LowerVolume.IA_LowerVolume"))
  (Class|BPIVolumeControl|ChangeVolume(Message) (Game|GetGameInstance) -0.1))

(event EventBeginPlay
  (bind _asplayer_controller (Utilities|Casting|CastToPlayerController (Pawn|GetController)))
  (Input|AddMappingContext (PlayerController|LocalPlayerSubsystems|GetEnhancedInputLocalPlayerSubsystem _asplayer_controller) "/Game/Input/Actions/IMC_Rhythm.IMC_Rhythm" 0 "(bIgnoreAllPressedKeysUntilRelease=True,bForceImmediately=False,bNotifyUserSettings=False)"))

(event Collision|EventActorBeginOverlap
  (params (OtherActor :type Actor%20Object%20Reference)))

(event EventTick
  (params (DeltaSeconds :type Float%20%28single-precision%29)))

(fn ConstructionScript)